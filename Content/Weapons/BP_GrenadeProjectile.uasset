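; Grenade projectile Blueprint that explodes on a short fixed fuse after spawning.
; BeginPlay waits on a Delay, then calls the Explode event.
; Explode spawns an explosion particle at the actor's location, applies radial damage sized by the DamageRadius variable and credited to the instigator's controller, then destroys the actor.
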(event `self.ReceiveBeginPlay`
  (`KismetSystemLibrary.Delay` 1.0)
  (`self.Explode`))

(event `Explode`
  (`GameplayStatics.SpawnEmitterAtLocation` "/Game/WeaponEffects/Explosion/P_Explosion.P_Explosion" (`self.K2_GetActorLocation`))
  (`GameplayStatics.ApplyRadialDamage` :`BaseDamage` 100.0 :`Origin` (`self.K2_GetActorLocation`) :`DamageRadius` (`self.DamageRadius`) :`DamageCauser` self :`InstigatedByController` (`self.GetInstigatorController`))
  (`self.K2_DestroyActor`))

(fn `UserConstructionScript`)