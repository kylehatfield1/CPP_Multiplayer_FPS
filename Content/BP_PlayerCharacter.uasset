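; BP_PlayerCharacter is the player character, armed with a launcher weapon and shown a crosshair on screen.
; On BeginPlay it spawns BP_LauncherWeapon with itself as owner and instigator, snaps it to the mesh's Weapon_r socket, and adds WBP_Crosshair to the viewport.
; Pressing the Fire input calls Fire on the stored weapon reference, leaving firing logic to the weapon.
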(event `self.ReceiveBeginPlay`
  (bind _returnvalue (`|SpawnActorFromClass` "/Game/BP_LauncherWeapon.BP_LauncherWeapon_C" (`KismetMathLibrary.MakeTransform` (0.0 0.0 0.0)) "AlwaysSpawn" "OverrideRootScale" self self))
  (bind _output_get (set `self.Weapon_ref` _returnvalue))
  (`self.K2_AttachToComponent` _output_get (`self.Mesh`) "Weapon_r" "SnapToTarget" "SnapToTarget" "SnapToTarget" true)
  (bind _returnvalue_2 (`|CreateWidget` "/Game/WBP_Crosshair.WBP_Crosshair_C"))
  (`UserWidget.AddToViewport` _returnvalue_2 0))

(event `InputAction|Fire`
  (params (Key :type "Key Structure"))
  (:`Pressed`
    (`Rifle.Fire` (`self.Weapon_ref`))))

(event `self.ReceiveTick`
  (params (DeltaSeconds :type "Float (single-precision)")))

(fn `UserConstructionScript`)